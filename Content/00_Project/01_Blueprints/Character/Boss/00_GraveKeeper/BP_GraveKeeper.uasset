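; GraveKeeper boss character that waits with movement disabled until BossDrop enables walking; BossBattleStart then clears the attacking state and starts BossFSMComponent.
; ExecuteBossPattern maps pattern names to Scratch, Crush, Bite and Dodge actions, played as animation overrides, with attacks setting IsAttacking.
; Scratch, Bite and Dodge report completion to the FSM, while Crush has no completion callback here.
; PlayDeathAnimation is an empty stub, and EventForTest enables walking and starts the FSM directly.
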(event Custom|Attack_Scratch
  ;[0.15 0.15 0.15 0.5] Boss Action Event
  (Development|PrintString "Scratch Called!")
  (|PlayAnimationOverridewithCallbacks (Variables|Default|GetBossAnimInstance) "/Game/00_Project/01_Blueprints/Character/Boss/00_GraveKeeper/AnimSequences/GraveKeeper_Scratch.GraveKeeper_Scratch" "DefaultSlot" 1.0 0.0
    (:then
      (Variables|Default|SetbIsAttacking true))
    (:OnCompleted
      (Class|BossFSMComponent|ActionFinished (Variables|Default|GetBossFSMComponent)))))

(event Custom|Attack_Crush
  ;[0.15 0.15 0.15 0.5] Boss Action Event
  (Development|PrintString "Crush Called!")
  (|PlayAnimationOverridewithCallbacks (Variables|Default|GetBossAnimInstance) "/Game/00_Project/01_Blueprints/Character/Boss/00_GraveKeeper/AnimSequences/GraveKeeper_Crush.GraveKeeper_Crush" "DefaultSlot" 1.0 0.0
    (:then
      (Variables|Default|SetbIsAttacking true))))

(event Custom|Attack_Bite
  ;[0.15 0.15 0.15 0.5] Boss Action Event
  (Development|PrintString "Bite Called!")
  (|PlayAnimationOverridewithCallbacks (Variables|Default|GetBossAnimInstance) "/Game/00_Project/01_Blueprints/Character/Boss/00_GraveKeeper/AnimSequences/GraveKeeper_Bite.GraveKeeper_Bite" "DefaultSlot" 1.0 0.0
    (:then
      (Variables|Default|SetbIsAttacking true))
    (:OnCompleted
      (Class|BossFSMComponent|ActionFinished (Variables|Default|GetBossFSMComponent)))))

(event Custom|EventForTest
  ;[0.15 0.15 0.15 0.5] Battle Start Sequence
  (Pawn|Components|CharacterMovement|SetMovementMode (Variables|Character|GetCharacterMovement) "MOVE_Walking" 0)
  (Class|DefaultCharBase|SetIsAttacking false)
  (Class|BossFSMComponent|StartFSM (Variables|Default|GetBossFSMComponent)))

(event Custom|Dodge_Dodge
  ;[0.15 0.15 0.15 0.5] Boss Action Event
  (Development|PrintString "Dodge Called!")
  (|PlayAnimationOverridewithCallbacks (Variables|Default|GetBossAnimInstance) "/Game/00_Project/01_Blueprints/Character/Boss/00_GraveKeeper/AnimSequences/GraveKeeper_Dodge.GraveKeeper_Dodge" "DefaultSlot" 1.0 0.0
    (:OnCompleted
      (Class|BossFSMComponent|ActionFinished (Variables|Default|GetBossFSMComponent)))))

(event Custom|BossBattleStart
  ;[0.15 0.15 0.15 0.5] Battle Start Sequence
  (Class|DefaultCharBase|SetIsAttacking false)
  (Class|BossFSMComponent|StartFSM (Variables|Default|GetBossFSMComponent)))

(event Custom|BossDrop
  ;[0.15 0.15 0.15 0.5] Battle Start Sequence
  (Pawn|Components|CharacterMovement|SetMovementMode (Variables|Character|GetCharacterMovement) "MOVE_Walking" 0)
  (Class|DefaultCharBase|SetIsAttacking true))

(event EventBeginPlay
  (|CallParentFunction)
  (Pawn|Components|CharacterMovement|SetMovementMode (Variables|Character|GetCharacterMovement) "MOVE_None" 0))

(event EventPlayDeathAnimation)

(event EventExecuteBossPattern
  (params (PatternName :type Name :default "None"))
  ;[0.15 0.15 0.15 0.5] Choose Action
  (switch name PatternName
    (:Scratch
      (CallFunction|AttackScratch))
    (:Crush
      (CallFunction|AttackCrush))
    (:Bite
      (CallFunction|AttackBite))
    (:Dodge
      (CallFunction|DodgeDodge))))

(fn ConstructionScript
  (|CallParentFunction))