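; BP_Player is the player character, handling input for X-axis movement, jumping and attacking.
; Possession and BeginPlay cache the player controller and animation instance.
; The overridden Attack calls its parent, then plays animation overrides: combo-indexed ground sequences that reset the combo on completion, or a jump attack while falling that ends the attack state.
; Move input also stores direction and vertical value for use elsewhere.
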(event Input|EnhancedActionEvents|EnhancedInputActionIA_Jump
  (params (ActionValue :type Boolean) (ElapsedSeconds :type Float%20%28double-precision%29) (TriggeredSeconds :type Float%20%28double-precision%29) (InputAction :type Input%20Action%20Object%20Reference :default "/Game/00_Project/02_Inputs/InputActions/IA_Jump.IA_Jump"))
  ;[0.15 0.15 0.15 0.5] PlayerJump
  (:Started
    (Class|PlayerBase|TryJump))
  (:Completed
    (Class|PlayerBase|TryStopJumping)))

(event Input|EnhancedActionEvents|EnhancedInputActionIA_Move
  (params (ActionValue :type Vector%202D%20Structure) (ElapsedSeconds :type Float%20%28double-precision%29) (TriggeredSeconds :type Float%20%28double-precision%29) (InputAction :type Input%20Action%20Object%20Reference :default "/Game/00_Project/02_Inputs/InputActions/IA_Move.IA_Move"))
  (bind (_x _y) (Math|Vector2D|BreakVector2D ActionValue))
  ;[0.15 0.15 0.15 0.5] Player X-Axis movement, save Y-Axis value for other functions
  (Variables|Default|SetDirectionality ActionValue)
  (Pawn|Input|AddMovementInput self "1.000000,0.000000,0.000000" _x false)
  (Variables|Default|SetVerticalInputValue _y))

(event Input|EnhancedActionEvents|EnhancedInputActionIA_DefaultAttack
  (params (ActionValue :type Boolean) (ElapsedSeconds :type Float%20%28double-precision%29) (TriggeredSeconds :type Float%20%28double-precision%29) (InputAction :type Input%20Action%20Object%20Reference :default "/Game/00_Project/02_Inputs/InputActions/IA_DefaultAttack.IA_DefaultAttack"))
  ;[0.15 0.15 0.15 0.5] Actual attack input action (Call actual "Attack" Event Function)
  (:Started
    (Class|DefaultCharBase|TryAttack)))

(event EventBeginPlay
  ;[0.15 0.15 0.15 0.5] Set player animation instance as variable
  (Variables|Default|SetPlayerAnimInstance (Variables|/Script/PaperZD.PaperZDAnimationComponent|GetAnimInstance (Variables|Default|GetAnimationComponent))))

(event Collision|EventActorBeginOverlap
  (params (OtherActor :type Actor%20Object%20Reference)))

(event EventAttack
  (bind _attackanimsequence (Variables|Default|GetAttackAnimSequence))
  ;[0.15 0.15 0.15 0.5] Set attack event
  (|CallParentFunction)
  (if (not (AI|Components|NavMovement|IsFalling (Variables|Character|GetCharacterMovement)))
    (|PlayAnimationOverridewithCallbacks (Variables|Default|GetPlayerAnimInstance) (Utilities|Array|Get(acopy) _attackanimsequence (Math|Integer|%(Integer) (Variables|Default|GetComboCount) (Utilities|Array|Length _attackanimsequence))) "DefaultSlot" 1.0 0.0
      (:OnCompleted
        (Class|PlayerBase|ResetCombo)))
    (else
      (|PlayAnimationOverridewithCallbacks (Variables|Default|GetPlayerAnimInstance) "/Game/00_Project/01_Blueprints/Character/Player/AnimSequences/Player_JumpAttack.Player_JumpAttack" "DefaultSlot" 1.0 0.0
        (:OnCompleted
          (Class|DefaultCharBase|EndAttackState))))))

(event EventPossessed
  (params (NewController :type Controller%20Object%20Reference))
  ;[0.15 0.15 0.15 0.5] Set playercontoller as variable
  (bind _asbp_player_controller (Utilities|Casting|CastToBP_PlayerController NewController))
  (Variables|Default|SetPlayerController _asbp_player_controller))

(fn ConstructionScript)