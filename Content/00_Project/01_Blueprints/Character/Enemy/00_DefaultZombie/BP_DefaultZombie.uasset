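; Default zombie enemy Blueprint that supplies the zombie-specific hit and attack animations to its parent enemy class.
; PlayHitAnimation plays the hit sequence as an animation override on the enemy AnimInstance.
; Attack runs the parent logic, then plays the attack override, signaling attack end to the simple FSM whether the animation completes or is cancelled.
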(event EventBeginPlay
  (|CallParentFunction) ; This node is disabled and will not be called.\nDrag off pins to build functionality.
)

(event Collision|EventActorBeginOverlap
  (params (OtherActor :type Actor%20Object%20Reference))
  (|CallParentFunction OtherActor) ; This node is disabled and will not be called.\nDrag off pins to build functionality.
)

(event EventTick
  (params (DeltaSeconds :type Float%20%28single-precision%29))
  (|CallParentFunction DeltaSeconds) ; This node is disabled and will not be called.\nDrag off pins to build functionality.
)

(event EventPlayHitAnimation
  ;[0.15 0.15 0.15 0.5] Play hit animation
  (|PlayAnimationOverridewithCallbacks (Variables|Default|GetEnemyAnimInstance) "/Game/00_Project/01_Blueprints/Character/Enemy/00_DefaultZombie/AnimSequences/DefaultZombie_Hit.DefaultZombie_Hit" "DefaultSlot" 1.0 0.0))

(event EventAttack
  ;[0.15 0.15 0.15 0.5] Attack Implemented sequence
  (|CallParentFunction)
  (|PlayAnimationOverridewithCallbacks (Variables|Default|GetEnemyAnimInstance) "/Game/00_Project/01_Blueprints/Character/Enemy/00_DefaultZombie/AnimSequences/DefaultZombie_Attack.DefaultZombie_Attack" "DefaultSlot" 1.0 0.0
    (:OnCompleted
      _)
    (:OnCancelled
      _))
  (Class|EnemyBase|CallAttackEndonSimpleFSM))

(fn ConstructionScript
  (|CallParentFunction))