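; Soldier enemy Blueprint that supplies soldier-specific hit, attack and death animations on top of its parent enemy class.
; Each animation event plays its sequence as an override on the enemy anim instance.
; Attack runs the parent logic first, then signals attack end to the simple FSM whether the animation completes or is cancelled.
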(event EventBeginPlay
  (|CallParentFunction) ; This node is disabled and will not be called.\nDrag off pins to build functionality.
)

(event Collision|EventActorBeginOverlap
  (params (OtherActor :type Actor%20Object%20Reference))
  (|CallParentFunction OtherActor) ; This node is disabled and will not be called.\nDrag off pins to build functionality.
)

(event EventTick
  (params (DeltaSeconds :type Float%20%28single-precision%29)))

(event EventPlayHitAnimation
  ;[0.15 0.15 0.15 0.5] Play hit animation
  (|PlayAnimationOverridewithCallbacks (Variables|Default|GetEnemyAnimInstance) "/Game/00_Project/01_Blueprints/Character/Enemy/02_Soldier/AnimSequences/Soldier_Hit.Soldier_Hit" "DefaultSlot" 1.0 0.0))

(event EventAttack
  ;[0.15 0.15 0.15 0.5] Attack Implemented sequence
  (|CallParentFunction)
  (|PlayAnimationOverridewithCallbacks (Variables|Default|GetEnemyAnimInstance) "/Game/00_Project/01_Blueprints/Character/Enemy/02_Soldier/AnimSequences/Soldier_Attack.Soldier_Attack" "DefaultSlot" 1.0 0.0
    (:OnCompleted
      _)
    (:OnCancelled
      _))
  (Development|PrintString "CallEndSoldierAttackState")
  (Class|EnemyBase|CallAttackEndonSimpleFSM))

(event EventPlayDeathAnimation
  ;[0.15 0.15 0.15 0.5] Death animation
  (|PlayAnimationOverridewithCallbacks (Variables|Default|GetEnemyAnimInstance) "/Game/00_Project/01_Blueprints/Character/Enemy/02_Soldier/AnimSequences/Soldier_Death.Soldier_Death" "DefaultSlot" 1.0 0.0
    (:then
      (Development|PrintString "Call Death Animation"))))

(fn ConstructionScript
  (|CallParentFunction))