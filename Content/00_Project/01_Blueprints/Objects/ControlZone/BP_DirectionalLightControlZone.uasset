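; BP_DirectionalLightControlZone is a trigger zone that changes the yaw of a target light when something begins overlapping it.
; On overlap it stores the light's current rotation and, if the yaw differs from TargetYaw, snaps to that yaw while keeping pitch and roll.
; A timeline-based blend over TransitionTime with shortest-path rotation interpolation is present but disconnected, so it never runs.
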(event OnComponentBeginOverlap(LightControlZone)
  (params (OverlappedComponent :type Primitive%20Component%20Object%20Reference) (OtherActor :type Actor%20Object%20Reference) (OtherComp :type Primitive%20Component%20Object%20Reference) (OtherBodyIndex :type Integer) (bFromSweep :type Boolean) (SweepResult :type Hit%20Result%20Structure%20%28by%20ref%29))
  (Variables|00_LightControl|SetOriginRotation (Transformation|GetActorRotation (Variables|00_LightControl|GetTargetLight)))
  (if (not (== (.yaw (Variables|00_LightControl|GetOriginRotation)) (Variables|00_LightControl|GetTargetYaw)))
    (Transformation|SetActorRotation (Variables|00_LightControl|GetTargetLight) (Math|Rotator|MakeRotator (.roll (Variables|00_LightControl|GetOriginRotation)) (.pitch (Variables|00_LightControl|GetOriginRotation)) (Variables|00_LightControl|GetTargetYaw)))))

(fn ConstructionScript)