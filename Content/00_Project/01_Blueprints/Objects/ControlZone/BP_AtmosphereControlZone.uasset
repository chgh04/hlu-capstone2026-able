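; BP_AtmosphereControlZone is a trigger zone that changes the level's lighting and fog when something overlaps its LightControlZone component.
; On overlap it snaps TargetLight to TargetYaw, keeping pitch and roll, with no filter on the overlapping actor.
; If ModifyFog is set, it also moves TargetFog to TargetFogZ in height.
; A timeline-based smooth rotation over TransitionTime exists but is disconnected, so changes are instant.
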(event OnComponentBeginOverlap(LightControlZone)
  (params (OverlappedComponent :type Primitive%20Component%20Object%20Reference) (OtherActor :type Actor%20Object%20Reference) (OtherComp :type Primitive%20Component%20Object%20Reference) (OtherBodyIndex :type Integer) (bFromSweep :type Boolean) (SweepResult :type Hit%20Result%20Structure%20%28by%20ref%29))
  (Utilities|FlowControl|Sequence
    (:then_0
      ;[0.15 0.15 0.15 0.5] Change Directional Light
      (Variables|00LightControl|SetOriginRotation (Transformation|GetActorRotation (Variables|00LightControl|GetTargetLight)))
      (if (not (== (.yaw (Variables|00LightControl|GetOriginRotation)) (Variables|00LightControl|GetTargetYaw)))
        (Transformation|SetActorRotation (Variables|00LightControl|GetTargetLight) (Math|Rotator|MakeRotator (.roll (Variables|00LightControl|GetOriginRotation)) (.pitch (Variables|00LightControl|GetOriginRotation)) (Variables|00LightControl|GetTargetYaw)))))
    (:then_1
      ;[0.15 0.15 0.15 0.5] Change Exponential Fog
      (if (Variables|01_FogControl|GetbModifyFog)
        (Variables|01_FogControl|SetOriginFogLocation (Transformation|GetActorLocation (Variables|01_FogControl|GetTargetFog)))
        (Transformation|SetActorLocation (Variables|01_FogControl|GetTargetFog) (Math|Vector|MakeVector (.x (Variables|01_FogControl|GetOriginFogLocation)) (.y (Variables|01_FogControl|GetOriginFogLocation)) (Variables|01_FogControl|GetTargetFogZ)) false false)))))

(fn ConstructionScript)