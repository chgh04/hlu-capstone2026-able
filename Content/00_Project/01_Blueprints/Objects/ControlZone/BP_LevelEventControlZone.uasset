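; Level event control zone that locks the player into an arena behind two blocking walls.
; Any overlap with the zone starts the arena once, enabling wall collision, firing the locked notification and fading the walls through dynamic materials on a timeline.
; DeactivateArena disables collision, runs a second fade timeline and fires the unlocked notification when it finishes.
; Within this graph, only TestEvent calls deactivation, and the started flag never resets.
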(event OnComponentBeginOverlap(EventControlZone)
  (params (OverlappedComponent :type Primitive%20Component%20Object%20Reference) (OtherActor :type Actor%20Object%20Reference) (OtherComp :type Primitive%20Component%20Object%20Reference) (OtherBodyIndex :type Integer) (bFromSweep :type Boolean) (SweepResult :type Hit%20Result%20Structure%20%28by%20ref%29))
  (CallFunction|ActiveArena))

(event Custom|ActiveArena
  ;[0.15 0.15 0.15 0.5] Start Arena Event
  (if (not (Variables|Default|GetbIsArenaStart))
    (Variables|Default|SetbIsArenaStart true)
    (Utilities|FlowControl|Sequence
      (:then_0
        (bind _returnvalue (Rendering|Material|CreateDynamicMaterialInstance (Variables|Default|GetBlockWall_1) 0 0 "None" :!class /Script/Engine.PrimitiveComponent))
        (Variables|Default|SetBlockWall_1_DynamicMT _returnvalue)
        (bind _returnvalue_2 (Rendering|Material|CreateDynamicMaterialInstance (Variables|Default|GetBlockWall_2) 0 0 "None" :!class /Script/Engine.PrimitiveComponent))
        (Variables|Default|SetBlockWall_2_DynamicMT _returnvalue_2))
      (:then_1
        (Collision|SetCollisionEnabled (Variables|Default|GetBlockWall_1) "QueryAndPhysics")
        (Collision|SetCollisionEnabled (Variables|Default|GetBlockWall_2) "QueryAndPhysics")
        (Default|CallOnArenaLocked))
      (:then_2
        (bind _alpha (Timeline|FadeWall PlayFromStart)
          (:Update
            (Rendering|Material|SetScalarParameterValue (Variables|Default|GetBlockWall_1_DynamicMT) "FadeAmount" _alpha :!class /Script/Engine.MaterialInstanceDynamic)
            (Rendering|Material|SetScalarParameterValue (Variables|Default|GetBlockWall_2_DynamicMT) "FadeAmount" _alpha :!class /Script/Engine.MaterialInstanceDynamic))
          (:Finished))))))

(event Custom|DeactivateArena
  ;[0.15 0.15 0.15 0.5] End Arena Event
  (Collision|SetCollisionEnabled (Variables|Default|GetBlockWall_1) "NoCollision")
  (Collision|SetCollisionEnabled (Variables|Default|GetBlockWall_2) "NoCollision")
  (bind _alpha (Timeline|RemoveWall Play)
    (:Update
      (Rendering|Material|SetScalarParameterValue (Variables|Default|GetBlockWall_1_DynamicMT) "FadeAmount" _alpha :!class /Script/Engine.MaterialInstanceDynamic)
      (Rendering|Material|SetScalarParameterValue (Variables|Default|GetBlockWall_2_DynamicMT) "FadeAmount" _alpha :!class /Script/Engine.MaterialInstanceDynamic))
    (:Finished
      (Default|CallOnArenaUnlocked))))

(event Custom|TestEvent
  (CallFunction|DeactivateArena))

(fn ConstructionScript)