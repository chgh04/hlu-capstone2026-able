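; BP_GroundFillControlZone is a trigger zone that swaps which ground fill objects are visible when something overlaps it.
; On begin overlap of its GroundFillControlZone component, it hides each valid actor in RemoveGroundFillObject, then shows each in AddGroundFillObject.
; It only toggles hidden-in-game state, with no filter on the overlapping actor and no revert on exit.
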(event OnComponentBeginOverlap(GroundFillControlZone)
  (params (OverlappedComponent :type Primitive%20Component%20Object%20Reference) (OtherActor :type Actor%20Object%20Reference) (OtherComp :type Primitive%20Component%20Object%20Reference) (OtherBodyIndex :type Integer) (bFromSweep :type Boolean) (SweepResult :type Hit%20Result%20Structure%20%28by%20ref%29))
  (Utilities|FlowControl|Sequence
    (:then_0
      (for _array_element (Variables|00_GorundFillObject|GetRemoveGroundFillObject)
        (if (Utilities|IsValid _array_element)
          (Rendering|SetActorHiddenInGame _array_element true))))
    (:then_1
      (for _array_element_2 (Variables|00_GorundFillObject|GetAddGroundFillObject)
        (if (Utilities|IsValid _array_element_2)
          (Rendering|SetActorHiddenInGame _array_element_2 false))))))

(fn ConstructionScript)