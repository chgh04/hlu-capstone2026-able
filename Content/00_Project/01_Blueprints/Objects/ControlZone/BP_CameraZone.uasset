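; BP_CameraZone is a trigger volume that changes the camera setup of actors that overlap it.
; On entry it messages the actor to use either a fixed camera or a new arm length and socket offset, and on exit it resets that.
; It can also override a target post-process volume's sensor width and focal distance, matching focus to the new arm length, caching the originals to restore on exit.
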(event OnComponentBeginOverlap(CameraControlZone)
  (params (OverlappedComponent :type Primitive%20Component%20Object%20Reference) (OtherActor :type Actor%20Object%20Reference) (OtherComp :type Primitive%20Component%20Object%20Reference) (OtherBodyIndex :type Integer) (bFromSweep :type Boolean) (SweepResult :type Hit%20Result%20Structure%20%28by%20ref%29))
  (bind _targetpostprocessvolume (Variables|01_PostProcessVolume|GetTargetPostProcessVolume))
  (Utilities|FlowControl|Sequence
    (:then_0
      ;[0.15 0.15 0.15 0.5] Set Camera Offset
      (if (Variables|00_Camera|GetbIsCamFixed)
        (Class|BPIPlayerCameraOffsetControl|FixedCameraSetting(Message) OtherActor self)
        (else
          (Class|BPIPlayerCameraOffsetControl|ChangeCameraSetting(Message) OtherActor (Variables|00_Camera|GetNewCameraArmLength) (Variables|00_Camera|GetNewCameraSocketOffset)))))
    (:then_1
      ;[0.15 0.15 0.15 0.5] Set Post Process Volume Settings
      (if (Variables|01_PostProcessVolume|GetbModifyPostProcess)
        (Utilities|IsValid _targetpostprocessvolume
          (:Is%20Valid
            (Variables|01_PostProcessVolume|SetOriginSensorWidth (.DepthOfFieldSensorWidth (Utilities|Struct|BreakPostProcessSettings (Variables|/Script/Engine.PostProcessVolume|GetSettings _targetpostprocessvolume))))
            (Variables|01_PostProcessVolume|SetOriginFocalDistnace (.DepthOfFieldFocalDistance (Utilities|Struct|BreakPostProcessSettings (Variables|/Script/Engine.PostProcessVolume|GetSettings _targetpostprocessvolume))))
            (bind _structout (Utilities|Struct|SetmembersinPostProcessSettings (Variables|/Script/Engine.PostProcessVolume|GetSettings (Variables|01_PostProcessVolume|GetTargetPostProcessVolume)) (Variables|01_PostProcessVolume|GetNewSensorWidth) (Variables|00_Camera|GetNewCameraArmLength)))
            (Variables|/Script/Engine.PostProcessVolume|SetSettings (Variables|01_PostProcessVolume|GetTargetPostProcessVolume) _structout)))))))

(event OnComponentEndOverlap(CameraControlZone)
  (params (OverlappedComponent :type Primitive%20Component%20Object%20Reference) (OtherActor :type Actor%20Object%20Reference) (OtherComp :type Primitive%20Component%20Object%20Reference) (OtherBodyIndex :type Integer))
  (bind _targetpostprocessvolume (Variables|01_PostProcessVolume|GetTargetPostProcessVolume))
  (Utilities|FlowControl|Sequence
    (:then_0
      ;[0.15 0.15 0.15 0.5] Reset Camera Offset
      (if (Variables|00_Camera|GetbIsCamFixed)
        (Class|BPIPlayerCameraOffsetControl|EndFixedCamSetting(Message) OtherActor)
        (else
          (Class|BPIPlayerCameraOffsetControl|ResetCameraSetting(Message) OtherActor))))
    (:then_1
      ;[0.15 0.15 0.15 0.5] Reset Post Process Volume Settings
      (if (Variables|01_PostProcessVolume|GetbModifyPostProcess)
        (Utilities|IsValid _targetpostprocessvolume
          (:Is%20Valid
            (bind _structout (Utilities|Struct|SetmembersinPostProcessSettings (Variables|/Script/Engine.PostProcessVolume|GetSettings _targetpostprocessvolume) (Variables|01_PostProcessVolume|GetOriginSensorWidth) (Variables|01_PostProcessVolume|GetOriginFocalDistnace)))
            (Variables|/Script/Engine.PostProcessVolume|SetSettings (Variables|01_PostProcessVolume|GetTargetPostProcessVolume) _structout)))))))

(fn ConstructionScript)