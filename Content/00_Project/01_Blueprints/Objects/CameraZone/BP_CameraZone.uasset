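; BP_CameraZone is a placeable volume that changes the camera behavior of actors overlapping its CameraControlZone component.
; On begin overlap, IsCamFixed selects between passing itself for a fixed-camera setup and sending a new arm length and socket offset.
; On end overlap, it sends the matching end or reset message.
; All changes go through interface messages to the overlapping actor, with no cast or actor filtering.
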(event OnComponentBeginOverlap(CameraControlZone)
  (params (OverlappedComponent :type Primitive%20Component%20Object%20Reference) (OtherActor :type Actor%20Object%20Reference) (OtherComp :type Primitive%20Component%20Object%20Reference) (OtherBodyIndex :type Integer) (bFromSweep :type Boolean) (SweepResult :type Hit%20Result%20Structure%20%28by%20ref%29))
  (if (Variables|00_Camera|GetbIsCamFixed)
    (Class|BPIPlayerCameraOffsetControl|FixedCameraSetting(Message) OtherActor self)
    (else
      (Class|BPIPlayerCameraOffsetControl|ChangeCameraSetting(Message) OtherActor (Variables|00_Camera|GetNewCameraArmLength) (Variables|00_Camera|GetNewCameraSocketOffset)))))

(event OnComponentEndOverlap(CameraControlZone)
  (params (OverlappedComponent :type Primitive%20Component%20Object%20Reference) (OtherActor :type Actor%20Object%20Reference) (OtherComp :type Primitive%20Component%20Object%20Reference) (OtherBodyIndex :type Integer))
  (if (Variables|00_Camera|GetbIsCamFixed)
    (Class|BPIPlayerCameraOffsetControl|EndFixedCamSetting(Message) OtherActor)
    (else
      (Class|BPIPlayerCameraOffsetControl|ResetCameraSetting(Message) OtherActor))))

(fn ConstructionScript)